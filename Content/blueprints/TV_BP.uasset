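; TV actor that the player toggles between viewing through a camera and normal third-person play via its Interactable event.
; A FlipFlop blends the view to the camera, clears widgets, locks movement and turning and shows the cursor, then reverses the view, lock and cursor on the next call.
; Tick re-fetches the CameraActor and BP_ThirdPersonCharacter view targets every frame with GetActorOfClass.
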(event `self.ReceiveTick`
  (params (DeltaSeconds :type "Float (single-precision)"))
  (`|ExecutionSequence`
    (:`then_0`
      (bind _returnvalue (`GameplayStatics.GetActorOfClass` "/Script/Engine.CameraActor"))
      (set `self.Camera` _returnvalue))
    (:`then_1`
      (bind _returnvalue_2 (`GameplayStatics.GetActorOfClass` "/Game/ThirdPerson/Blueprints/BP_ThirdPersonCharacter.BP_ThirdPersonCharacter_C"))
      (set `self.Main` _returnvalue_2))))

(event `/Game/Interaction/InteractionInterface.Interactable`
  (bind _returnvalue (`GameplayStatics.GetPlayerController` 0))
  (`/Engine/EditorBlueprintResources/StandardMacros.FlipFlop`
    (:`A`
      (set `self.isLooking` true)
      (`WidgetLayoutLibrary.RemoveAllWidgets`)
      (`KismetSystemLibrary.PrintString` "looking")
      (`PlayerController.SetViewTargetWithBlend` _returnvalue (`self.Camera`) 0.5 "VTBlend_Linear" 0.0 false)
      (`PlayerController.SetCinematicMode` _returnvalue true true true true true)
      (set `PlayerController.bShowMouseCursor` true _returnvalue)
      (`WidgetBlueprintLibrary.SetInputMode_GameAndUIEx` _returnvalue null "LockOnCapture"))
    (:`B`
      (set `self.isLooking` false)
      (`KismetSystemLibrary.PrintString` "not looking")
      (`PlayerController.SetViewTargetWithBlend` _returnvalue (`self.main`) 0.5 "VTBlend_Linear" 0.0 false)
      (`PlayerController.SetCinematicMode` _returnvalue false true true true true)
      (set `PlayerController.bShowMouseCursor` false _returnvalue)
      (`WidgetBlueprintLibrary.SetInputMode_GameOnly` _returnvalue))))

(fn `UserConstructionScript`)